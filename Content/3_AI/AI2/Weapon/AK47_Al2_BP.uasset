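; AK47 weapon Blueprint for an AI, apparently adapted from a player weapon, with most of its logic disconnected.
; Fire, stop, reload and unequip events are empty; the gated auto-fire loop, montage reload, camera-based spread trace and magazine refill are unreachable, player-dependent leftovers.
; AmmoCheck still decrements ammo and plays a randomized shot sound, and GunLight switches on the muzzle flash.
; SpawnDecalTracer's spawning is unwired, so it spawns nothing.
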(event Custom|Event%20Fire%20Base
  ;[1 1 1] Fire
)

(event Custom|Event%20Stop%20Fire
  ;[1 1 1] Fire
)

(event Custom|Event%20Un%20eqiup
  ;[1 1 1] Comment
)

(event Custom|Event%20Reload%20Base
  ;[1 1 1] Reload
)

(fn ConstructionScript)

(fn AmmoCheck
  (bind _returnvalue (Math|Random|RandomFloatinRange 0.7 1.2))
  (Math|Integer|DecrementInt (Variables|Default|GetAmmo_Count)
    (:%20%20
      (Audio|PlaySoundatLocation 0 (Transformation|GetActorLocation) "0, 0, 0" (* _returnvalue 2.5) _returnvalue 0.0 0 0 0)
      (return))))

(fn LineTrace)

(fn SpawnDecalTracer
  (params (SpawnTransform :type Vector) (ImpactPoint :type Vector))
  (if (not (>= (Math|Random|RandomIntegerinRange 1 10) 0))
    (return)))

(fn UpdateAmmo)