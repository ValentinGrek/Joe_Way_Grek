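; AI controller for the AI2 enemy that runs the BT_Perception behavior tree and shoots at sensed characters.
; Perception writes or clears the Player blackboard key, caches stimulus locations and toggles PersonTarget for ThirdPersonCharacter targets.
; Tick requests player prediction and, while targeting, uses a Delay to pace FireAndDistance, which spawns bullets from the pawn's arrow within Radius.
; The target death check is disconnected and never runs.
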(event OnTargetPerceptionUpdated(AIPerception)
  (params (Actor :type Actor%20Object%20Reference) (Stimulus :type AI%20Stimulus%20Structure))
  (bind _returnvalue (Utilities|String|StringToName "Player"))
  (bind _blackboard (Variables|Default|GetBlackboard))
  (if (.bSuccessfullySensed (Utilities|Struct|BreakAIStimulus Stimulus))
    (AI|Components|Blackboard|SetValueasObject _blackboard _returnvalue Actor)
    (else
      (AI|Components|Blackboard|ClearValue _blackboard _returnvalue))))

(event OnTargetPerceptionInfoUpdated(AIPerception)
  (params (UpdateInfo :type Actor%20Perception%20Update%20Info%20Structure%20%28by%20ref%29))
  (Variables|Default|SetUpdate%20Info%20Stimulus%20Stimulus%20Location (.stimuluslocation (.stimulus UpdateInfo)))
  (Variables|Default|SetUpdate%20Info%20Stimulus%20Receiver%20Location (.receiverlocation (.stimulus UpdateInfo)))
  (bind _asthird_person_character (Utilities|Casting|CastToThirdPersonCharacter (.target UpdateInfo)))
  (if (Variables|Default|GetPersonTarget)
    (Variables|Default|SetPersonTarget false)
    (else
      (Variables|Default|SetPersonTarget true))))

(event EventBeginPlay
  (AI|RunBehaviorTree "/Game/3_AI/AI2/Blueprints/BT_Perception.BT_Perception"))

(event EventTick
  (params (DeltaSeconds :type Float%20%28single-precision%29))
  (Class|AISensePrediction|RequestControllerPredictionEvent self (Game|Player|GetPlayerPawn 0) 0.5)
  (if (Variables|Default|GetPersonTarget)
    (bind _asai2_bp_new (Utilities|Casting|CastToAI2_BP (Pawn|GetControlledPawn)))
    (Utilities|FlowControl|Delay 0.15)
    (CallFunction|FireandDistance (Variables|Default|GetUpdate%20Info%20Stimulus%20Stimulus%20Location) (Variables|Default|GetUpdate%20Info%20Stimulus%20Receiver%20Location) _asai2_bp_new)))

(fn ConstructionScript)

(fn FireandDistance
  (params (Actor%20Loc :type Vector) (AI2%20Loc :type Vector) (AI2_BP_New :type AI2%20BP%20Object%20Reference))
  (LocalVariables|SetAI2%20BP%20New AI2_BP_New)
  (if (< (Math|Vector|Distance(Vector) Actor%20Loc AI2%20Loc) (Variables|Default|GetRadius))
    (Game|SpawnActorfromClass "/Game/3_AI/AI1/Bullet_AI1.Bullet_AI1_C" (Math|Transform|MakeTransform (Transformation|GetWorldLocation (Variables|/Game/3_AI/AI2/Blueprints/AI2_BP.AI2_BP_C|GetArrow1 (LocalVariables|GetAI2%20BP%20New))) (Transformation|GetWorldRotation (Variables|/Game/3_AI/AI2/Blueprints/AI2_BP.AI2_BP_C|GetArrow1 (LocalVariables|GetAI2%20BP%20New))) "0.500000,0.500000,0.500000") "Undefined" 0 0)
    (Audio|PlaySoundatLocation "/Game/2_Weapon/Sounds/DryFire.DryFire" (Transformation|GetActorLocation (LocalVariables|GetAI2%20BP%20New)) "0, 0, 0" 1.0 1.0 0.0 0 0 0)))