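; BP_Target2 is a shootable target that holds an AK47, shows an HP bar and dies when its health runs out.
; On BeginPlay it links itself to the HP widget and attaches a spawned rifle to the mesh's Weapon socket.
; Tick turns the bar toward the player's follow camera.
; BulletAK47 overlaps reduce HP, playing a hit reaction or a one-time death that hides the bar, then destroys rifle and target after a delay.
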(event OnComponentBeginOverlap(Mesh)
  (params (OverlappedComponent :type Primitive%20Component%20Object%20Reference) (OtherActor :type Actor%20Object%20Reference) (OtherComp :type Primitive%20Component%20Object%20Reference) (OtherBodyIndex :type Integer) (bFromSweep :type Boolean) (SweepResult :type Hit%20Result%20Structure%20%28by%20ref%29))
  ;[1 0.0331 0] Урон и смерть
  (if (> (Variables|Default|GetHP) 0.0)
    (bind _asbullet_ak47 (Utilities|Casting|CastToBulletAK47 OtherActor))
    (Variables|Default|SetHP (- (Variables|Default|GetHP) (Variables|/Game/2_Weapon/Blueprints/Tracers/BulletAK47.BulletAK47_C|GetDamage _asbullet_ak47)))
    (if (> (Variables|Default|GetHP) 0.0)
      (Components|Animation|PlayAnimation (Variables|Character|GetMesh) "/Game/Mannequin/Animations/Animations/UseWeapon/Sequence/Hit_React_3_3.Hit_React_3_3" false)
      (else
        (if (not (Variables|Default|GetDeath)) :!label _label
          (Variables|Default|SetDeath true)
          (Rendering|SetVisibility (Variables|Default|GetHR%20Bar) false false)
          (Components|Animation|PlayAnimation (Variables|Character|GetMesh) "/Game/Mannequin/Animations/Animations/UseWeapon/Sequence/Death_3_3.Death_3_3" false)
          (Utilities|FlowControl|Delay 5.0)
          (Actor|DestroyActor (Variables|Default|GetAk47_Weapon)))))
    (else
      (goto _label))))

(event EventTick
  (params (DeltaSeconds :type Float%20%28single-precision%29))
  (bind _returnvalue (Game|Player|GetPlayerPawn 0))
  (bind _hr_bar (Variables|Default|GetHR%20Bar))
  (bind _asthird_person_character (Utilities|Casting|CastToThirdPersonCharacter _returnvalue))
  ;[1 1 1] Поворот виджета к персонажу
  (Utilities|IsValid _hr_bar
    (:Is%20Valid
      (Utilities|IsValid _asthird_person_character
        (:Is%20Valid
          (Transformation|SetWorldRotation _hr_bar (Math|Rotator|FindLookatRotation (Transformation|GetWorldLocation _hr_bar) (Transformation|GetWorldLocation (Variables|/Game/ThirdPersonBP/Blueprints/ThirdPersonCharacter.ThirdPersonCharacter_C|GetFollowCamera _asthird_person_character))) false false))))))

(event EventBeginPlay
  ;[1 1 1] Связать виджет с actor
  (bind _asw_hp_bar_target_2 (Utilities|Casting|CastToW_HP_Bar_Target2 (UserInterface|GetUserWidgetObject (Variables|Default|GetHR%20Bar))))
  (Variables|/Game/2_Targets/Target2/W_HP_Bar_Target2.W_HP_Bar_Target2_C|SetTarget2 _asw_hp_bar_target_2 self)
  (bind _returnvalue (Game|SpawnActorfromClass "/Game/2_Weapon/Blueprints/BP_Weapon_AK47.BP_Weapon_AK47_C" (Math|Transform|MakeTransform "0, 0, 0" "0, 0, 0" "1,1,1") "AlwaysSpawn" 0 0))
  (bind _output_get (Variables|Default|SetAk47_Weapon _returnvalue))
  (Transformation|AttachComponentToComponent _output_get (Variables|Character|GetMesh) "Weapon" "SnapToTarget" "SnapToTarget" "SnapToTarget" true))

(fn ConstructionScript)