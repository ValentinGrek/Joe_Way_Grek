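; Player inventory Blueprint that stores item classes and amounts in a slot array, sized on a new game and exportable as a save struct.
; On BeginPlay it creates a hidden inventory widget on the main HUD canvas, toggled by status alongside cursor and input mode.
; AddItem merges stackable items into matching slots or uses the last empty one, refreshes that slot's widget and returns a result enum.
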(event EventBeginPlay
  (switch Utilities|FlowControl|Switch|SwitchonE_InventoryStartMode (Variables|Default|GetStart%20Mode)
    (:NewEnumerator0
      (Utilities|Array|Resize (Variables|Default|GetSlots) (Variables|Default|GetAmount%20Of%20Slots))
      (CallFunction|CreateInventoryWidject))
    (:NewEnumerator1
      (CallFunction|CreateInventoryWidject))))

(fn ConstructionScript)

(fn GetSaveData
  (return (Utilities|Struct|MakeS_SaveInventoryInfo (Variables|Default|GetAmount%20Of%20Slots) (Variables|Default|GetSlots))))

(fn GetSlotInfofromIndex
  (params (Index :type Integer))
  (bind _slots (Variables|Default|GetSlots))
  (bind _output (Utilities|Array|Get(acopy) _slots Index))
  (bind (_item _amount) (Utilities|Struct|BreakS_Slot_Structure _output))
  (if (Utilities|IsValidClass _item)
    ;[0.000611 1 0] Если слот не пустой - записываем данные
    (return false (.ItemStructure (Utilities|GetClassDefaults _item)) _amount)
    (else
      ;[1 0 0.01502] Если слот пустой - выдаем пустой
      (return true "" 0))))

(fn CreateInventoryWidject
  (bind _returnvalue (Viewport|GetViewportSize))
  (bind _returnvalue_2 (UserInterface|CreateWidget "/Game/4_Inventory/Widjets/Inv_WB.Inv_WB_C" 0 self))
  (bind _output_get (Variables|Default|SetInv%20WB%20Ref _returnvalue_2))
  (Widget|SetVisibility _output_get "Hidden")
  ;[1 1 1] Добавляем инвентарь на экран
  (bind _returnvalue_3 (Class|CanvasPanel|AddChildtoCanvas (Variables|/Game/ThirdPersonBP/Blueprints/Widjets/Main_HUD.Main_HUD_C|GetCanvasPanel_0 (Variables|Default|GetMain%20HUD%20Ref)) _returnvalue_2))
  (Class|CanvasPanelSlot|SetAutoSize _returnvalue_3 true)
  (Class|CanvasPanelSlot|SetPosition _returnvalue_3 (Math|Vector2D|MakeVector2D (/ (.x _returnvalue) 1.3) (/ (.y _returnvalue) 2.0)))
  (return))

(fn ShowInventory
  (Utilities|IsValid (Variables|Default|GetInv%20WB%20Ref)
    (:Is%20Valid
      (switch Utilities|FlowControl|Switch|SwitchonE_InventoryStatus (Variables|Default|GetStatus)
        (:NewEnumerator2
          (Widget|SetVisibility (Variables|Default|GetInv%20WB%20Ref) "Visible")
          (Variables|/Script/Engine.PlayerController|SetbShowMouseCursor (Game|GetPlayerController 0) true)
          (Input|SetInputModeGameandUI (Game|GetPlayerController 0) (Variables|Default|GetMain%20HUD%20Ref) "DoNotLock" false)
          (Variables|Default|SetStatus "NewEnumerator3")
          (return))))))

(fn HideInventory
  (Utilities|IsValid (Variables|Default|GetInv%20WB%20Ref)
    (:Is%20Valid
      (switch Utilities|FlowControl|Switch|SwitchonE_InventoryStatus (Variables|Default|GetStatus)
        (:NewEnumerator3
          (Widget|SetVisibility (Variables|Default|GetInv%20WB%20Ref) "Hidden")
          (if (Variables|/Game/ThirdPersonBP/Blueprints/ThirdPersonCharacter.ThirdPersonCharacter_C|GetDeath (.AsThird%20Person%20Character (Utilities|Casting|CastToThirdPersonCharacter (Game|GetPlayerCharacter 0))))
            _
            (else
              (Variables|/Script/Engine.PlayerController|SetbShowMouseCursor (Game|GetPlayerController 0) false)))
          (Input|SetInputModeGameOnly (Game|GetPlayerController 0))
          (Variables|Default|SetStatus "NewEnumerator2")
          (return))))))

(fn HideShowInventoryFlipFlop
  (switch Utilities|FlowControl|Switch|SwitchonE_InventoryStatus (Variables|Default|GetStatus)
    (:NewEnumerator2
      (HideShowInventory|ShowInventory))
    (:NewEnumerator3
      (HideShowInventory|HideInventory))))

(fn UpdateSlot
  (params (Index :type Integer))
  (Default|UpdateSlot (Utilities|Array|Get(acopy) (Variables|/Game/4_Inventory/Widjets/Inv_WB.Inv_WB_C|GetSlot%20Widjets%20Array (Variables|Default|GetInv%20WB%20Ref)) Index)))

(fn SearchEmptySlot
  (bind (_array_element _array_index) (Utilities|Array|ForEachLoopwithBreak (Variables|Default|GetSlots))
    (:LoopBody
      (if (not (Utilities|IsValidClass (.Item (Utilities|Struct|BreakS_Slot_Structure _array_element))))
        (LocalVariables|SetLocal%20Boolean true)
        (LocalVariables|SetLocal%20Index _array_index)))
    (:Completed
      (return (LocalVariables|GetLocal%20Boolean) (LocalVariables|GetLocal%20Index)))))

(fn SearchSlotIndexforStack
  (params (Item :type BP%20Pick%20Base%20Class%20Reference))
  (bind (_array_element _array_index) (Utilities|Array|ForEachLoopwithBreak (Variables|Default|GetSlots) :!label _label)
    (:LoopBody
      (if (and (Utilities|IsValidClass (.Item (Utilities|Struct|BreakS_Slot_Structure _array_element))) (== (.Item (Utilities|Struct|BreakS_Slot_Structure _array_element)) Item))
        (LocalVariables|SetLocal%20Stack%20Is%20Founded true)
        (goto _label Break)))
    (:Completed
      (return (LocalVariables|GetLocal%20Stack%20Is%20Founded) _array_index))))

(fn AddItem
  (params (Item :type BP%20Pick%20Base%20Class%20Reference) (Amount :type Integer))
  (LocalVariables|SetLocal%20Item Item)
  (bind _output_get (LocalVariables|SetLocal%20Amount Amount))
  (if (> _output_get 0)
    (if (.stacked (.ItemStructure (Utilities|GetClassDefaults (LocalVariables|GetLocal%20Item))))
      ;[1 1 1] Новый слот или пристакать?
      (bind (_succsess _founded_index) (CallFunction|SearchSlotIndexforStack (LocalVariables|GetLocal%20Item)))
      (if _succsess
        ;[1 1 1] Стакаем одинаковые предметы вместе
        (Utilities|Array|SetArrayElem (Variables|Default|GetSlots) _founded_index (Utilities|Struct|MakeS_Slot_Structure (LocalVariables|GetLocal%20Item) (+ (.amount (Utilities|Array|Get(acopy) (Variables|Default|GetSlots) _founded_index)) (LocalVariables|GetLocal%20Amount))))
        ;[1 1 1] Обновляем слоты
        (CallFunction|UpdateSlot _founded_index)
        ;[0.03382 1 0] Предмет пристакан
        (return true "NewEnumerator1")
        (else
          _)))
    ;[1 1 1] Поиск пустого слота
    (bind (_succsess_2 _index) (CallFunction|SearchEmptySlot))
    (if _succsess_2
      ;[1 1 1] Добавляем предмет в инвентарь
      (Utilities|Array|SetArrayElem (Variables|Default|GetSlots) _index (Utilities|Struct|MakeS_Slot_Structure (LocalVariables|GetLocal%20Item) (LocalVariables|GetLocal%20Amount)))
      ;[1 1 1] Обновляем слоты
      (CallFunction|UpdateSlot _index)
      ;[0.03382 1 0] Предмет добавлен
      (return true "NewEnumerator0")
      (else
        ;[1 0 0.001865] Нет места в инвентаре
        (return false "NewEnumerator2")))))